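; Dialogue component for Wiglaf's birthday conversation, where he reminds Beowulf of his big day and asks him to hand out invitations.
; Overrides Dialogue, calls the parent, then switches on DialogueTreeIndex, with only index 0 handled.
; That branch is a linear chain of AddDialogue calls with a single Continue option and a shared talking animation, voice audio on Wiglaf's lines, and CloseConvo at the end.
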(fn `dialogue`
  (`parent.dialogue`)
  (switch `int` (`self.dialogueTreeIndex`)
    (:`0`
      (bind _state (`self.Add Dialogue` "Wiglaf" "Hey Beowulf!" (`|MakeArray` "Continue" :!type "Text") "/Game/Audio/VoiceLines/wiglaf/wiglaf-21.wiglaf-21" "/Game/NPCs/friends/THEKING/HrothgarTalking_InFront.HrothgarTalking_InFront"))
      (switch `/Game/dialogueSystem/Enum_Dialogue_State` _state
        (:`NewEnumerator0`
          (bind _state_2 (`self.Add Dialogue` "Beowulf" "*nods*" (`|MakeArray` "Continue" :!type "Text") null "/Game/NPCs/friends/THEKING/HrothgarTalking_InFront.HrothgarTalking_InFront"))
          (bind _state_3 (`self.Add Dialogue` "Beowulf" "*sighs*" (`|MakeArray` "Continue" :!type "Text") null "/Game/NPCs/friends/THEKING/HrothgarTalking_InFront.HrothgarTalking_InFront"))
          (bind _state_4 (`self.Add Dialogue` "Wiglaf" " Do you know what day it is Beowulf! It’s the big day! " (`|MakeArray` "Continue" :!type "Text") "/Game/Audio/VoiceLines/wiglaf/wiglaf-22.wiglaf-22" "/Game/NPCs/friends/THEKING/HrothgarTalking_InFront.HrothgarTalking_InFront"))
          (switch `/Game/dialogueSystem/Enum_Dialogue_State` _state_4
            (:`NewEnumerator0`
              (bind _state_5 (`self.Add Dialogue` "Beowulf" "Ohhh yeahhhhh…" (`|MakeArray` "Continue" :!type "Text") null "/Game/NPCs/friends/THEKING/HrothgarTalking_InFront.HrothgarTalking_InFront"))
              (switch `/Game/dialogueSystem/Enum_Dialogue_State` _state_5
                (:`NewEnumerator0`
                  (bind _state_6 (`self.Add Dialogue` "Beowulf" "The tavern’s half off today isn’t it?" (`|MakeArray` "Continue" :!type "Text") null "/Game/NPCs/friends/THEKING/HrothgarTalking_InFront.HrothgarTalking_InFront"))
                  (switch `/Game/dialogueSystem/Enum_Dialogue_State` _state_6
                    (:`NewEnumerator0`
                      (bind _state_7 (`self.Add Dialogue` "Wiglaf" "Nooo!!! Don’t be silly, you know what day it is." (`|MakeArray` "Continue" :!type "Text") "/Game/Audio/VoiceLines/wiglaf/wiglaf-23.wiglaf-23" "/Game/NPCs/friends/THEKING/HrothgarTalking_InFront.HrothgarTalking_InFront"))
                      (switch `/Game/dialogueSystem/Enum_Dialogue_State` _state_7
                        (:`NewEnumerator0`
                          (bind _state_8 (`self.Add Dialogue` "Wiglaf" "Right? " (`|MakeArray` "Continue" :!type "Text") "/Game/Audio/VoiceLines/wiglaf/wiglaf-24.wiglaf-24" "/Game/NPCs/friends/THEKING/HrothgarTalking_InFront.HrothgarTalking_InFront"))
                          (switch `/Game/dialogueSystem/Enum_Dialogue_State` _state_8
                            (:`NewEnumerator0`
                              (bind _state_9 (`self.Add Dialogue` "Beowulf" "?" (`|MakeArray` "Continue" :!type "Text") null "/Game/NPCs/friends/THEKING/HrothgarTalking_InFront.HrothgarTalking_InFront"))
                              (switch `/Game/dialogueSystem/Enum_Dialogue_State` _state_9
                                (:`NewEnumerator0`
                                  (bind _state_10 (`self.Add Dialogue` "Wiglaf" " MY BIRTHDAY!  " (`|MakeArray` "Continue" :!type "Text") "/Game/Audio/VoiceLines/wiglaf/wiglaf-25.wiglaf-25" "/Game/NPCs/friends/THEKING/HrothgarTalking_InFront.HrothgarTalking_InFront"))
                                  (switch `/Game/dialogueSystem/Enum_Dialogue_State` _state_10
                                    (:`NewEnumerator0`
                                      (bind _state_11 (`self.Add Dialogue` "Beowulf" "Oh- Of course, Of course how could I forget… Your birthday  ! Yeahhhh! \n" (`|MakeArray` "Continue" :!type "Text") null "/Game/NPCs/friends/THEKING/HrothgarTalking_InFront.HrothgarTalking_InFront"))
                                      (switch `/Game/dialogueSystem/Enum_Dialogue_State` _state_11
                                        (:`NewEnumerator0`
                                          (bind _state_12 (`self.Add Dialogue` "Wiglaf" "Oh boy, it’s gonna be amazing! " (`|MakeArray` "Continue" :!type "Text") "/Game/Audio/VoiceLines/wiglaf/wiglaf-27.wiglaf-27" "/Game/NPCs/friends/THEKING/HrothgarTalking_InFront.HrothgarTalking_InFront"))
                                          (switch `/Game/dialogueSystem/Enum_Dialogue_State` _state_12
                                            (:`NewEnumerator0`
                                              (bind _state_13 (`self.Add Dialogue` "Wiglaf" "I'm gonna have a feast meant for kings!" (`|MakeArray` "Continue" :!type "Text") "/Game/Audio/VoiceLines/wiglaf/wiglaf-27.wiglaf-27" "/Game/NPCs/friends/THEKING/HrothgarTalking_InFront.HrothgarTalking_InFront"))
                                              (switch `/Game/dialogueSystem/Enum_Dialogue_State` _state_13
                                                (:`NewEnumerator0`
                                                  (bind _state_14 (`self.Add Dialogue` "Wiglaf" "Alcohol flowing like a river!" (`|MakeArray` "Continue" :!type "Text") "/Game/Audio/VoiceLines/wiglaf/wiglaf-28.wiglaf-28" "/Game/NPCs/friends/THEKING/HrothgarTalking_InFront.HrothgarTalking_InFront"))
                                                  (switch `/Game/dialogueSystem/Enum_Dialogue_State` _state_14
                                                    (:`NewEnumerator0`
                                                      (bind _state_15 (`self.Add Dialogue` "Wiglaf" "But most importantly! I will be with my favorite people!" (`|MakeArray` "Continue" :!type "Text") "/Game/Audio/VoiceLines/wiglaf/wiglaf-29.wiglaf-29" "/Game/NPCs/friends/THEKING/HrothgarTalking_InFront.HrothgarTalking_InFront"))
                                                      (switch `/Game/dialogueSystem/Enum_Dialogue_State` _state_15
                                                        (:`NewEnumerator0`
                                                          (bind _state_16 (`self.Add Dialogue` "Beowulf" "Thas crazy" (`|MakeArray` "Continue" :!type "Text") null "/Game/NPCs/friends/THEKING/HrothgarTalking_InFront.HrothgarTalking_InFront"))
                                                          (switch `/Game/dialogueSystem/Enum_Dialogue_State` _state_16
                                                            (:`NewEnumerator0`
                                                              (bind _state_17 (`self.Add Dialogue` "Wiglaf" "Beowulf, my greatest bestest friend, can you help me spread the word about my birthday?" (`|MakeArray` "Continue" :!type "Text") "/Game/Audio/VoiceLines/wiglaf/wiglaf-30.wiglaf-30" "/Game/NPCs/friends/THEKING/HrothgarTalking_InFront.HrothgarTalking_InFront"))
                                                              (switch `/Game/dialogueSystem/Enum_Dialogue_State` _state_17
                                                                (:`NewEnumerator0`
                                                                  (bind _state_18 (`self.Add Dialogue` "Wiglaf" "I went out a few days ago, knocking on everyone’s door, but I think everyone must of been busy that day cause no one came out . I’m gonna have to prioritize planning THE GREATEST, COOLEST, CRAZIEST birthday party Herot has ever seen!" (`|MakeArray` "Continue" :!type "Text") "/Game/Audio/VoiceLines/wiglaf/wiglaf-31.wiglaf-31" "/Game/NPCs/friends/THEKING/HrothgarTalking_InFront.HrothgarTalking_InFront"))
                                                                  (switch `/Game/dialogueSystem/Enum_Dialogue_State` _state_18
                                                                    (:`NewEnumerator0`
                                                                      (bind _state_19 (`self.Add Dialogue` "Beowulf" "Ughhh  *grumbles*" (`|MakeArray` "Continue" :!type "Text") null "/Game/NPCs/friends/THEKING/HrothgarTalking_InFront.HrothgarTalking_InFront"))
                                                                      (switch `/Game/dialogueSystem/Enum_Dialogue_State` _state_19
                                                                        (:`NewEnumerator0`
                                                                          (bind _state_20 (`self.Add Dialogue` "Beowulf" "Sure thing, Wiglaf, I’ll make sure everybody knows about it \n" (`|MakeArray` "Continue" :!type "Text") null "/Game/NPCs/friends/THEKING/HrothgarTalking_InFront.HrothgarTalking_InFront"))
                                                                          (switch `/Game/dialogueSystem/Enum_Dialogue_State` _state_20
                                                                            (:`NewEnumerator0`
                                                                              (bind _state_21 (`self.Add Dialogue` "Wiglaf" "Thank you friend. I’m gonna start preparing right now       \n" (`|MakeArray` "Continue" :!type "Text") "/Game/Audio/VoiceLines/wiglaf/wiglaf-32.wiglaf-32" "/Game/NPCs/friends/THEKING/HrothgarTalking_InFront.HrothgarTalking_InFront"))
                                                                              (switch `/Game/dialogueSystem/Enum_Dialogue_State` _state_21
                                                                                (:`NewEnumerator0`
                                                                                  (`self.Add Dialogue` "Wiglaf" "Here are some invitations you can hand out! See you in a few hours!" (`|MakeArray` "Continue" :!type "Text") "/Game/Audio/VoiceLines/wiglaf/wiglaf-33.wiglaf-33" "/Game/NPCs/friends/THEKING/HrothgarTalking_InFront.HrothgarTalking_InFront")
                                                                                  (`self.closeConvo`))))))))))))))))))))))))))))))))))))))))))