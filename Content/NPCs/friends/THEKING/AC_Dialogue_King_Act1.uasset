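; Dialogue component for King Hrothgar in Act 1, scripting his throne room conversations with Beowulf and Sir Aeschere.
; A saved tree index picks the branch, advancing from 1 to 2 once Grendel is dead.
; Chained AddDialogue calls supply text, options, voice audio and animations targeting the king or knight mesh.
; In the opening, refusing the quest triggers KillBeowulf, while accepting sends Aeschere away and opens a looping question menu.
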(fn `dialogue`
  (set `self.kingAnimationSkeleton` (`Actor.GetComponentByClass` (`self.GetOwner`) "/Script/Engine.SkeletalMeshComponent"))
  (`parent.dialogue`)
  (bind _returnvalue (`GameplayStatics.GetActorOfClass` "/Game/NPCs/friends/Wiglaf/NPC_Wiglaf.NPC_Wiglaf_C"))
  (bind _returnvalue_2 (`GameplayStatics.GetActorOfClass` "/Game/NPCs/foes/GrendelMother/GRENDELMOMMEADHALL.GRENDELMOMMEADHALL_C"))
  (bind _returnvalue_3 (`GameplayStatics.GetActorOfClass` "/Game/dialogueSystem/NPC_Base.NPC_Base_C"))
  (bind _asnpc_knight (cast `/Game/NPCs/friends/Aeschere/NPC_Knight` _returnvalue_3))
  (bind _asbp_first_person_character (cast `/Game/Dynamic/FirstPerson/Blueprints/BP_FirstPersonCharacter` (`GameplayStatics.GetPlayerCharacter` 0)))
  (bind _game_mode (`/Game/Dynamic/FirstPerson/Blueprints/BP_FirstPersonCharacter.Game Mode` _asbp_first_person_character))
  (bind _as_level_save_data (`/Game/Dynamic/FirstPerson/Blueprints/BP_FirstPersonGameMode.As Level Save Data` _game_mode))
  (set `self.dialogueTreeIndex` (`/Game/Dynamic/FirstPerson/Blueprints/levelSaveData.kingDialogueTreeIndex` _as_level_save_data))
  (set `self.knightAnimationSkeleton` (`Character.Mesh` _asnpc_knight))
  (if (and (`/Game/Dynamic/FirstPerson/Blueprints/levelSaveData.grendelDead?` _as_level_save_data) (== (`self.dialogueTreeIndex`) 1))
    (set `self.dialogueTreeIndex` 2))
  (switch `int` (`self.dialogueTreeIndex`)
    (:`0`
      (bind _state (`self.Add Dialogue` "Beowulf" "*Yawn*  Yeah, that was a splendid nap. Oh what's going on here..." (`|MakeArray` "Continue" :!type "Text") null "/Game/NPCs/friends/THEKING/HrothgarTalking_InFront.HrothgarTalking_InFront" (`self.kingAnimationSkeleton`)))
      (switch `/Game/dialogueSystem/Enum_Dialogue_State` _state
        (:`NewEnumerator0`
          (bind _state_2 (`self.Add Dialogue` "King Hrothgar" "What does thy mean thine forces is not great enough to defeat one measly goblin!" (`|MakeArray` "Continue" :!type "Text") "/Game/Audio/VoiceLines/KingHrothgar/king-01.king-01" "/Game/NPCs/friends/THEKING/HrothgarDisbeliefHeadDownn.HrothgarDisbeliefHeadDownn" (`self.kingAnimationSkeleton`)))
          (switch `/Game/dialogueSystem/Enum_Dialogue_State` _state_2
            (:`NewEnumerator0`
              (bind _state_3 (`self.Add Dialogue` "Sir Aeschere" "My lord, every platoon we sent out has yet to return. This foul beast hath massacared many of mine best knights." (`|MakeArray` "Continue" :!type "Text") "/Game/Audio/InStudioDialogue/Aeschere/New_Recording_143-converted.New_Recording_143-converted" "/Game/NPCs/friends/Aeschere/knight_talk_To_King.knight_talk_To_King" (`self.knightAnimationSkeleton`)))
              (switch `/Game/dialogueSystem/Enum_Dialogue_State` _state_3
                (:`NewEnumerator0`
                  (bind _state_4 (`self.Add Dialogue` "Sir Aeschere" "The kingdom's subjects are taking note of the bloodshed, and are beginning to lose faith in you my liege.  Thine goblin has become a matter of uptmost importance. " (`|MakeArray` "Continue" :!type "Text") "/Game/Audio/InStudioDialogue/Aeschere/New_Recording_144-converted.New_Recording_144-converted" "/Game/NPCs/friends/Aeschere/knight_look_To_King.knight_look_To_King" (`self.knightAnimationSkeleton`)))
                  (switch `/Game/dialogueSystem/Enum_Dialogue_State` _state_4
                    (:`NewEnumerator0`
                      (bind _state_5 (`self.Add Dialogue` "King Hrothgar" "So what does thine, suppose I do? " (`|MakeArray` "Continue" :!type "Text") "/Game/Audio/VoiceLines/KingHrothgar/king-02.king-02" "/Game/NPCs/friends/THEKING/HrothgarTalking_InFront.HrothgarTalking_InFront" (`self.kingAnimationSkeleton`)))
                      (switch `/Game/dialogueSystem/Enum_Dialogue_State` _state_5
                        (:`NewEnumerator0`
                          (bind _state_6 (`self.Add Dialogue` "Sir Aeschere" "My lord, I propose we lay an ambush for the beast by luring it near our castle walls and then- " (`|MakeArray` "Continue" :!type "Text") "/Game/Audio/InStudioDialogue/Aeschere/New_Recording_145-converted.New_Recording_145-converted" "/Game/NPCs/friends/Aeschere/knight_talk_To_King.knight_talk_To_King" (`self.knightAnimationSkeleton`)))
                          (switch `/Game/dialogueSystem/Enum_Dialogue_State` _state_6
                            (:`NewEnumerator0`
                              (bind _state_7 (`self.Add Dialogue` "Sir Aeschere" "What the!" (`|MakeArray` "Continue" :!type "Text") "/Game/Audio/InStudioDialogue/Aeschere/New_Recording_146-converted.New_Recording_146-converted" "/Game/NPCs/friends/Aeschere/knight_Notice_beowulf.knight_Notice_beowulf" (`self.knightAnimationSkeleton`)))
                              (switch `/Game/dialogueSystem/Enum_Dialogue_State` _state_7
                                (:`NewEnumerator0`
                                  (bind _state_8 (`self.Add Dialogue` "King Hrothgar" "Forsooth, I say! Spit it out Aeschere! " (`|MakeArray` "Continue" :!type "Text") "/Game/Audio/VoiceLines/KingHrothgar/king-03.king-03"))
                                  (switch `/Game/dialogueSystem/Enum_Dialogue_State` _state_8
                                    (:`NewEnumerator0`
                                      (bind _state_9 (`self.Add Dialogue` "Sir Aeschere" "Forgive my inquiry my lord, but wherefore is thither a peasant living in thine royal throneroom? " (`|MakeArray` "Continue" :!type "Text") "/Game/Audio/InStudioDialogue/Aeschere/New_Recording_147-converted.New_Recording_147-converted" "/Game/NPCs/friends/Aeschere/knight_Notice_lookKing.knight_Notice_lookKing" (`self.knightAnimationSkeleton`)))
                                      (switch `/Game/dialogueSystem/Enum_Dialogue_State` _state_9
                                        (:`NewEnumerator0`
                                          (bind _state_10 (`self.Add Dialogue` "King Hrothgar" "What is thou mumbling about- Oh." (`|MakeArray` "Continue" :!type "Text") "/Game/Audio/VoiceLines/KingHrothgar/king-04.king-04" "/Game/NPCs/friends/THEKING/Hrothgar_LookAtBeowulf.Hrothgar_LookAtBeowulf" (`self.kingAnimationSkeleton`)))
                                          (switch `/Game/dialogueSystem/Enum_Dialogue_State` _state_10
                                            (:`NewEnumerator0`
                                              (bind _state_11 (`self.Add Dialogue` "King Hrothgar" "What the devils! Who let this riffraff inside my royal castle!" (`|MakeArray` "Continue" :!type "Text") "/Game/Audio/VoiceLines/KingHrothgar/king-05.king-05" "/Game/NPCs/friends/Aeschere/knight_Notice_beowulf.knight_Notice_beowulf" (`self.knightAnimationSkeleton`)))
                                              (switch `/Game/dialogueSystem/Enum_Dialogue_State` _state_11
                                                (:`NewEnumerator0`
                                                  (bind _state_12 (`self.Add Dialogue` "Sir Aeschere" "Wish for me to dispose of this one, my king?" (`|MakeArray` "Continue" :!type "Text") "/Game/Audio/InStudioDialogue/Aeschere/New_Recording_148-converted.New_Recording_148-converted" "/Game/NPCs/friends/Aeschere/knight_Notice_lookKing.knight_Notice_lookKing" (`self.knightAnimationSkeleton`)))
                                                  (switch `/Game/dialogueSystem/Enum_Dialogue_State` _state_12
                                                    (:`NewEnumerator0`
                                                      (bind _state_13 (`self.Add Dialogue` "King Hrothgar" "Stand down, Aeschere! Hmmm. What an interesting one..." (`|MakeArray` "Continue" :!type "Text") "/Game/Audio/VoiceLines/KingHrothgar/king-06.king-06" "/Game/NPCs/friends/Aeschere/knight_Notice_beowulf.knight_Notice_beowulf" (`self.knightAnimationSkeleton`)))
                                                      (switch `/Game/dialogueSystem/Enum_Dialogue_State` _state_13
                                                        (:`NewEnumerator0`
                                                          (bind _state_14 (`self.Add Dialogue` "King Hrothgar" "You there! You seem like you have quite the build, hath you experience with the blade?" (`|MakeArray` "Continue" :!type "Text") "/Game/Audio/VoiceLines/KingHrothgar/king-07.king-07"))
                                                          (switch `/Game/dialogueSystem/Enum_Dialogue_State` _state_14
                                                            (:`NewEnumerator0`
                                                              (bind _state_15 (`self.Add Dialogue` "Beowulf" "Yep." (`|MakeArray` "Continue" :!type "Text")))
                                                              (switch `/Game/dialogueSystem/Enum_Dialogue_State` _state_15
                                                                (:`NewEnumerator0`
                                                                  (bind _state_16 (`self.Add Dialogue` "King Hrothgar" "Then I shall make you a knight of my kingdom! It is with great honor for you to obey the royal decree of......" (`|MakeArray` "Continue" :!type "Text") "/Game/Audio/VoiceLines/KingHrothgar/king-08.king-08"))
                                                                  (switch `/Game/dialogueSystem/Enum_Dialogue_State` _state_16
                                                                    (:`NewEnumerator0`
                                                                      (bind _state_17 (`self.Add Dialogue` "King Hrothgar" "Killing the ugly troll living in a shack across the road." (`|MakeArray` "Continue" :!type "Text") "/Game/Audio/VoiceLines/KingHrothgar/king-09.king-09"))
                                                                      (switch `/Game/dialogueSystem/Enum_Dialogue_State` _state_17
                                                                        (:`NewEnumerator0`
                                                                          (bind _state_18 (`self.Add Dialogue` "Beowulf" "Sure, I don't see why not." (`|MakeArray` "Continue" :!type "Text")))
                                                                          (switch `/Game/dialogueSystem/Enum_Dialogue_State` _state_18
                                                                            (:`NewEnumerator0`
                                                                              (bind _state_19 (`self.Add Dialogue` "Sir Aeschere" "Wha? Wh-Why??? Who?!??" (`|MakeArray` "Continue" :!type "Text") "/Game/Audio/InStudioDialogue/Aeschere/New_Recording_149-converted.New_Recording_149-converted" "/Game/NPCs/friends/Aeschere/knight_Disbelief.knight_Disbelief" (`self.knightAnimationSkeleton`)))
                                                                              (switch `/Game/dialogueSystem/Enum_Dialogue_State` _state_19
                                                                                (:`NewEnumerator0`
                                                                                  (bind _state_20 (`self.Add Dialogue` "King Hrothgar" "Is something the matter, Aeschere?" (`|MakeArray` "Continue" :!type "Text") "/Game/Audio/VoiceLines/KingHrothgar/king-10.king-10" "/Game/NPCs/friends/THEKING/HrothgarTalking_InFront.HrothgarTalking_InFront" (`self.kingAnimationSkeleton`)))
                                                                                  (switch `/Game/dialogueSystem/Enum_Dialogue_State` _state_20
                                                                                    (:`NewEnumerator0`
                                                                                      (bind _state_21 (`self.Add Dialogue` "Sir Aeschere" "My lord, in my 21 years on this Earth serving under your command, I have not once questioned your leadership, but....this, is er- unprecedented. May I implore why him?" (`|MakeArray` "Continue" :!type "Text") "/Game/Audio/InStudioDialogue/Aeschere/New_Recording_150-converted.New_Recording_150-converted" "/Game/NPCs/friends/Aeschere/knight_look_To_King.knight_look_To_King" (`self.knightAnimationSkeleton`)))
                                                                                      (switch `/Game/dialogueSystem/Enum_Dialogue_State` _state_21
                                                                                        (:`NewEnumerator0`
                                                                                          (bind _state_22 (`self.Add Dialogue` "King Hrothgar" "This peasant had the bravery to sleep in my throneroom with so much skill that not even my best knight could've detected him momentarily. I adore his moxie." (`|MakeArray` "Continue" :!type "Text") "/Game/Audio/VoiceLines/KingHrothgar/king-11.king-11" "/Game/NPCs/friends/THEKING/Hrothgar_LookAtBeowulf.Hrothgar_LookAtBeowulf" (`self.kingAnimationSkeleton`)))
                                                                                          (switch `/Game/dialogueSystem/Enum_Dialogue_State` _state_22
                                                                                            (:`NewEnumerator0`
                                                                                              (bind _state_23 (`self.Add Dialogue` "Sir Aeschere" "This is tomfoolery to the upmost extent! Thine doesn't even know if thy is skillful enough for such a beast! " (`|MakeArray` "Continue" :!type "Text") "/Game/Audio/InStudioDialogue/Aeschere/New_Recording_151-converted.New_Recording_151-converted" "/Game/NPCs/friends/Aeschere/knight_Disbelief.knight_Disbelief" (`self.knightAnimationSkeleton`)))
                                                                                              (switch `/Game/dialogueSystem/Enum_Dialogue_State` _state_23
                                                                                                (:`NewEnumerator0`
                                                                                                  (bind _state_24 (`self.Add Dialogue` "King Hrothgar" "Settle down, Aeschere! Forsooth, he said he is experienced with the blade himself, for he must be a natural! For this fact alone, I trust him with mine life." (`|MakeArray` "Continue" :!type "Text") "/Game/Audio/VoiceLines/KingHrothgar/king-12.king-12" "/Game/NPCs/friends/THEKING/HrothgarTalking_InFront.HrothgarTalking_InFront" (`self.kingAnimationSkeleton`)))
                                                                                                  (switch `/Game/dialogueSystem/Enum_Dialogue_State` _state_24
                                                                                                    (:`NewEnumerator0`
                                                                                                      (bind _state_25 (`self.Add Dialogue` "Sir Aeschere" "My lord..." (`|MakeArray` "Continue" :!type "Text") "/Game/Audio/InStudioDialogue/Aeschere/New_Recording_152-converted.New_Recording_152-converted" "/Game/NPCs/friends/Aeschere/knight_Notice_beowulf.knight_Notice_beowulf" (`self.knightAnimationSkeleton`)))
                                                                                                      (switch `/Game/dialogueSystem/Enum_Dialogue_State` _state_25
                                                                                                        (:`NewEnumerator0`
                                                                                                          (bind (_state_26 _optionindex) (`self.Add Dialogue` "King Hrothgar" "What do you say peasant? Will you take the quest to strike down this foul, grotesque, smelly,  ugly, heinous, and downright despicable beast that has been terrorizing our kingdom for millennia?" (`|MakeArray` "I changed my mind." "GIVE ME BLOOD!" :!type "Text") "/Game/Audio/VoiceLines/KingHrothgar/king-13.king-13" "/Game/NPCs/friends/THEKING/Hrothgar_LookAtBeowulf.Hrothgar_LookAtBeowulf" (`self.kingAnimationSkeleton`)))
                                                                                                          (switch `/Game/dialogueSystem/Enum_Dialogue_State` _state_26
                                                                                                            (:`NewEnumerator0`
                                                                                                              (switch `int` _optionindex
                                                                                                                (:`0`
                                                                                                                  (bind _state_27 (`self.Add Dialogue` "King Hrothgar" "Y'know what, I changed MY mind. Aeschere, kill him." (`|MakeArray` "Continue" :!type "Text") "/Game/Audio/VoiceLines/KingHrothgar/king-14.king-14" "/Game/NPCs/friends/THEKING/HrothgarTalking_InFront.HrothgarTalking_InFront" (`self.kingAnimationSkeleton`)))
                                                                                                                  (switch `/Game/dialogueSystem/Enum_Dialogue_State` _state_27
                                                                                                                    (:`NewEnumerator0`
                                                                                                                      (bind _state_28 (`self.Add Dialogue` "Sir Aeschere" "At your command, my liege." (`|MakeArray` "Continue" :!type "Text") "/Game/Audio/InStudioDialogue/Aeschere/New_Recording_153-converted.New_Recording_153-converted" "/Game/NPCs/friends/THEKING/Hrothgar_LookAtBeowulf.Hrothgar_LookAtBeowulf" (`self.kingAnimationSkeleton`)))
                                                                                                                      (switch `/Game/dialogueSystem/Enum_Dialogue_State` _state_28
                                                                                                                        (:`NewEnumerator0`
                                                                                                                          (`self.clearDialogueProgress`)
                                                                                                                          (`self.closeConvo`)
                                                                                                                          (`/Game/NPCs/friends/Aeschere/NPC_Knight.killBeowulf` _asnpc_knight))))))
                                                                                                                (:`1`
                                                                                                                  (bind _state_29 (`self.Add Dialogue` "King Hrothgar" "See Aeschere? This man is more than capable of battling that foul beast! If you're still not convinced then how bout' you test his ability in the training grounds? Eh Aeschere?" (`|MakeArray` "Continue" :!type "Text") "/Game/Audio/VoiceLines/KingHrothgar/king-15.king-15" "/Game/NPCs/friends/THEKING/HrothgarTalking_InFront.HrothgarTalking_InFront" (`self.kingAnimationSkeleton`)))
                                                                                                                  (switch `/Game/dialogueSystem/Enum_Dialogue_State` _state_29
                                                                                                                    (:`NewEnumerator0`
                                                                                                                      (bind _state_30 (`self.Add Dialogue` "Sir Aeschere" "I-Uh, suppose it wouldn't be fatal to inquire his combative ability." (`|MakeArray` "Continue" :!type "Text") "/Game/Audio/InStudioDialogue/Aeschere/New_Recording_154-converted.New_Recording_154-converted" "/Game/NPCs/friends/Aeschere/knight_Notice_lookKing.knight_Notice_lookKing" (`self.knightAnimationSkeleton`)))
                                                                                                                      (switch `/Game/dialogueSystem/Enum_Dialogue_State` _state_30
                                                                                                                        (:`NewEnumerator0`
                                                                                                                          (bind _state_31 (`self.Add Dialogue` "Sir Aeschere" "Peasant,  if you wish to test your ability, meet me in the training grounds to the left when you exit the royal castle, I'll be waiting." (`|MakeArray` "Continue" :!type "Text") "/Game/Audio/InStudioDialogue/Aeschere/New_Recording_155-converted.New_Recording_155-converted" "/Game/NPCs/friends/Aeschere/knight_Notice_beowulf.knight_Notice_beowulf" (`self.knightAnimationSkeleton`)))
                                                                                                                          (switch `/Game/dialogueSystem/Enum_Dialogue_State` _state_31
                                                                                                                            (:`NewEnumerator0`
                                                                                                                              (bind _state_32 (`self.Add Dialogue` "Sir Aeschere" "I just might be able to teach you a thing or two." (`|MakeArray` "Continue" :!type "Text") "/Game/Audio/InStudioDialogue/Aeschere/New_Recording_156-converted.New_Recording_156-converted" "/Game/NPCs/friends/THEKING/HrothgarTalking_InFront.HrothgarTalking_InFront" (`self.kingAnimationSkeleton`)))
                                                                                                                              (switch `/Game/dialogueSystem/Enum_Dialogue_State` _state_32
                                                                                                                                (:`NewEnumerator0`
                                                                                                                                  (if (not (`self.sceneAction`))
                                                                                                                                    (`/Game/NPCs/friends/Aeschere/NPC_Knight.knightWalkAway` _asnpc_knight)
                                                                                                                                    (set `self.sceneAction` true))
                                                                                                                                  (bind (_state_33 _optionindex_2) (`self.Add Dialogue` "King Hrothgar" "I suppose now would be the time to ask questions if you hath any." (`|MakeArray` "Why is a troll killing your villagers?" "How long has Grendel been attacking you?" "What's the deal with Aeschere?" "I don't have any questions." :!type "Text") "/Game/Audio/VoiceLines/KingHrothgar/king-16.king-16" "/Game/NPCs/friends/THEKING/HrothgarTalking_InFront.HrothgarTalking_InFront" (`self.kingAnimationSkeleton`) :!label _label))
                                                                                                                                  (switch `/Game/dialogueSystem/Enum_Dialogue_State` _state_33
                                                                                                                                    (:`NewEnumerator0`
                                                                                                                                      (switch `int` _optionindex_2
                                                                                                                                        (:`0`
                                                                                                                                          (bind _state_34 (`self.Add Dialogue` "King Hrothgar" "Why? WHY? Does an evil beast need a reason to commit heinous acts? I think not!" (`|MakeArray` "Continue" :!type "Text") "/Game/Audio/VoiceLines/KingHrothgar/king-17.king-17"))
                                                                                                                                          (switch `/Game/dialogueSystem/Enum_Dialogue_State` _state_34
                                                                                                                                            (:`NewEnumerator0`
                                                                                                                                              (bind _state_35 (`self.Add Dialogue` "King Hrothgar" "He is a monster, he is vile, and I hate his stupid face!" (`|MakeArray` "Continue" :!type "Text") "/Game/Audio/VoiceLines/KingHrothgar/king-18.king-18"))
                                                                                                                                              (switch `/Game/dialogueSystem/Enum_Dialogue_State` _state_35
                                                                                                                                                (:`NewEnumerator0`
                                                                                                                                                  (bind _state_36 (`self.Add Dialogue` "King Hrothgar" "All you need to know is that he is the scum of the earth and cannot be trusted." (`|MakeArray` "Continue" :!type "Text") "/Game/Audio/VoiceLines/KingHrothgar/king-19.king-19"))
                                                                                                                                                  (switch `/Game/dialogueSystem/Enum_Dialogue_State` _state_36
                                                                                                                                                    (:`NewEnumerator0`
                                                                                                                                                      (goto _label))))))))
                                                                                                                                        (:`1`
                                                                                                                                          (bind _state_37 (`self.Add Dialogue` "King Hrothgar" "The beast has been attacking our people for months now. Every week it seems as if someone new goes missing. " (`|MakeArray` "Continue" :!type "Text") "/Game/Audio/VoiceLines/KingHrothgar/king-20.king-20"))
                                                                                                                                          (switch `/Game/dialogueSystem/Enum_Dialogue_State` _state_37
                                                                                                                                            (:`NewEnumerator0`
                                                                                                                                              (bind _state_38 (`self.Add Dialogue` "King Hrothgar" "We sent out many knights to kill him, but as you can see, he got the better of them." (`|MakeArray` "Continue" :!type "Text") "/Game/Audio/VoiceLines/KingHrothgar/king-21.king-21"))
                                                                                                                                              (switch `/Game/dialogueSystem/Enum_Dialogue_State` _state_38
                                                                                                                                                (:`NewEnumerator0`
                                                                                                                                                  (bind _state_39 (`self.Add Dialogue` "King Hrothgar" "The latest attack,  was on the village near the marsh, the biome that of Grendel's own home. " (`|MakeArray` "Continue" :!type "Text") "/Game/Audio/VoiceLines/KingHrothgar/king-22.king-22"))
                                                                                                                                                  (switch `/Game/dialogueSystem/Enum_Dialogue_State` _state_39
                                                                                                                                                    (:`NewEnumerator0`
                                                                                                                                                      (bind _state_40 (`self.Add Dialogue` "King Hrothgar" "I reccommend you ask the townsfolk there questions on the beast, maybe their information could prove valuable." (`|MakeArray` "Continue" :!type "Text") "/Game/Audio/VoiceLines/KingHrothgar/king-23.king-23"))
                                                                                                                                                      (switch `/Game/dialogueSystem/Enum_Dialogue_State` _state_40
                                                                                                                                                        (:`NewEnumerator0`
                                                                                                                                                          (goto _label))))))))))
                                                                                                                                        (:`2`
                                                                                                                                          (bind _state_41 (`self.Add Dialogue` "King Hrothgar" "Ah, fret not peasant! Aeschere is simply worried of your wellbeing. Grendel is afterall, the biggest threat the Kingdom of the Danes, it is understandable he would be upset at the thought of sending a weakli- I mean strong dirt farmer to such peril." (`|MakeArray` "Continue" :!type "Text") "/Game/Audio/VoiceLines/KingHrothgar/king-24.king-24"))
                                                                                                                                          (switch `/Game/dialogueSystem/Enum_Dialogue_State` _state_41
                                                                                                                                            (:`NewEnumerator0`
                                                                                                                                              (bind _state_42 (`self.Add Dialogue` "King Hrothgar" "Just recently, he has been diagnosed with the rare condition called ethics, which was only just discovered by our court mages. We can only hope his condition doesn't worsen." (`|MakeArray` "Continue" :!type "Text") "/Game/Audio/VoiceLines/KingHrothgar/king-25.king-25"))
                                                                                                                                              (switch `/Game/dialogueSystem/Enum_Dialogue_State` _state_42
                                                                                                                                                (:`NewEnumerator0`
                                                                                                                                                  (bind _state_43 (`self.Add Dialogue` "King Hrothgar" "Aside, he hath been by mine side for a millenia, ever since he was a young boy as a matter of fact." (`|MakeArray` "Continue" :!type "Text") "/Game/Audio/VoiceLines/KingHrothgar/king-26.king-26"))
                                                                                                                                                  (switch `/Game/dialogueSystem/Enum_Dialogue_State` _state_43
                                                                                                                                                    (:`NewEnumerator0`
                                                                                                                                                      (bind _state_44 (`self.Add Dialogue` "King Hrothgar" "You may see why he may be careful when dealing with 'new blood', as he puts it." (`|MakeArray` "Continue" :!type "Text") "/Game/Audio/VoiceLines/KingHrothgar/king-27.king-27"))
                                                                                                                                                      (switch `/Game/dialogueSystem/Enum_Dialogue_State` _state_44
                                                                                                                                                        (:`NewEnumerator0`
                                                                                                                                                          (goto _label))))))))))
                                                                                                                                        (:`3`
                                                                                                                                          (bind _state_45 (`self.Add Dialogue` "King Hrothgar" "Well, off you go now! Don't make your king wait..." (`|MakeArray` "Continue" :!type "Text") "/Game/Audio/VoiceLines/KingHrothgar/king-28.king-28"))
                                                                                                                                          (switch `/Game/dialogueSystem/Enum_Dialogue_State` _state_45
                                                                                                                                            (:`NewEnumerator0`
                                                                                                                                              (`self.setDialogueTreeIndex` 1)
                                                                                                                                              (`self.clearDialogueProgress`)
                                                                                                                                              (`self.closeConvo`)
                                                                                                                                              (`CharacterMovementComponent.SetMovementMode` (`Character.CharacterMovement` _asbp_first_person_character) "MOVE_Walking" 0)
                                                                                                                                              (set `/Game/Dynamic/FirstPerson/Blueprints/BP_FirstPersonCharacter.isIdle` false _asbp_first_person_character)
                                                                                                                                              (`/Game/NPCs/friends/Aeschere/NPC_Knight.moveToTrainingGrounds` _asnpc_knight)
                                                                                                                                              (bind _output_get (set `/Game/Dynamic/FirstPerson/Blueprints/levelSaveData.kingDialogueTreeIndex` 1 _as_level_save_data))
                                                                                                                                              (set `self.dialogueTreeIndex` _output_get)
                                                                                                                                              (set `self.sceneAction` false))))))))))))))))))))))))))))))))))))))))))))))))))))))))))))))))))))))
    (:`1`
      (goto _label))
    (:`2`
      (bind _returnvalue_4 (`GameplayStatics.GetActorOfClass` "/Script/Engine.CameraActor"))
      (`PlayerController.SetViewTargetWithBlend` (`GameplayStatics.GetPlayerController` 0) _returnvalue_4 0.0 "VTBlend_Linear" 0.0 false)
      (bind _state_46 (`self.Add Dialogue` "King Hrothgar" "*While eating* Hehehe hah, so you see Aeschere, that’s why I say “Never let the peasantry rest easy”. Ahhhh… I then proceeded to order their execution shortly thereafter!" (`|MakeArray` "Continue" :!type "Text") "/Game/Audio/VoiceLines/KingHrothgar/king-29.king-29" "/Game/NPCs/friends/THEKING/Hrothgar_LookAtBeowulf.Hrothgar_LookAtBeowulf" (`self.knightAnimationSkeleton`)))
      (switch `/Game/dialogueSystem/Enum_Dialogue_State` _state_46
        (:`NewEnumerator0`
          (bind _state_47 (`self.Add Dialogue` "Sir Aeschere" "Wow, just wow, I don’t even know what to say to that.." (`|MakeArray` "Continue" :!type "Text") null "/Game/NPCs/friends/THEKING/HrothgarTalking_InFront.HrothgarTalking_InFront"))
          (switch `/Game/dialogueSystem/Enum_Dialogue_State` _state_47
            (:`NewEnumerator0`
              (bind _state_48 (`self.Add Dialogue` "Sir Aeschere" "Oh, It’s Beowulf! Glad to see that you came back in one piece! So how was it, was he toug-" (`|MakeArray` "Continue" :!type "Text") null "/Game/NPCs/friends/THEKING/HrothgarTalking_InFront.HrothgarTalking_InFront"))
              (switch `/Game/dialogueSystem/Enum_Dialogue_State` _state_48
                (:`NewEnumerator0`
                  (bind _state_49 (`self.Add Dialogue` "King Hrothgar" "*Spits out food* HOLY MACARONI! HOW ARE YOU NOT DEAD!" (`|MakeArray` "Continue" :!type "Text") "/Game/Audio/VoiceLines/KingHrothgar/king-30.king-30" "/Game/NPCs/friends/THEKING/HrothgarTalking_InFront.HrothgarTalking_InFront"))
                  (switch `/Game/dialogueSystem/Enum_Dialogue_State` _state_49
                    (:`NewEnumerator0`
                      (bind _state_50 (`self.Add Dialogue` "Sir Aeschere" "My liege, I am stumped. You sent him out predicting him to succeed, yes?" (`|MakeArray` "Continue" :!type "Text") null "/Game/NPCs/friends/THEKING/HrothgarTalking_InFront.HrothgarTalking_InFront" (`self.kingAnimationSkeleton`)))
                      (switch `/Game/dialogueSystem/Enum_Dialogue_State` _state_50
                        (:`NewEnumerator0`
                          (bind _state_51 (`self.Add Dialogue` "King Hrothgar" " W-Why of course, Aeschere! I would never send a peasant to die for my own amusement! What kind of man do you take your king to be?!" (`|MakeArray` "Continue" :!type "Text") "/Game/Audio/VoiceLines/KingHrothgar/king-31.king-31" "/Game/NPCs/friends/THEKING/HrothgarTalking_InFront.HrothgarTalking_InFront"))
                          (switch `/Game/dialogueSystem/Enum_Dialogue_State` _state_51
                            (:`NewEnumerator0`
                              (bind _state_52 (`self.Add Dialogue` "Sir Aeschere" "Just a second ago you sounded surpri-" (`|MakeArray` "Continue" :!type "Text") null "/Game/NPCs/friends/THEKING/HrothgarTalking_InFront.HrothgarTalking_InFront"))
                              (switch `/Game/dialogueSystem/Enum_Dialogue_State` _state_52
                                (:`NewEnumerator0`
                                  (bind _state_53 (`self.Add Dialogue` "King Hrothgar" "SSHHHH!" (`|MakeArray` "Continue" :!type "Text") "/Game/Audio/VoiceLines/KingHrothgar/king-32.king-32" "/Game/NPCs/friends/THEKING/HrothgarTalking_InFront.HrothgarTalking_InFront"))
                                  (switch `/Game/dialogueSystem/Enum_Dialogue_State` _state_53
                                    (:`NewEnumerator0`
                                      (if (not (`self.sceneAction`))
                                        (`SceneComponent.K2_SetWorldLocation` (`Character.CapsuleComponent` _returnvalue) (-15983.704597 -31953.397706 200.0) false true)
                                        (`/Game/NPCs/friends/Wiglaf/NPC_Wiglaf.meadACT2WalkIn` _returnvalue)
                                        (set `self.sceneAction` true))
                                      (bind _state_54 (`self.Add Dialogue` "Wiglaf" "King, sir! I have successfully relayed your message to Beowul- Oh! You’re already here! Hello sir Beowulf!" (`|MakeArray` "Continue" :!type "Text") "/Game/Audio/VoiceLines/wiglaf/wiglaf-06.wiglaf-06" "/Game/NPCs/friends/THEKING/HrothgarTalking_InFront.HrothgarTalking_InFront"))
                                      (switch `/Game/dialogueSystem/Enum_Dialogue_State` _state_54
                                        (:`NewEnumerator0`
                                          (bind _state_55 (`self.Add Dialogue` "Beowulf" "Sup." (`|MakeArray` "Continue" :!type "Text") null "/Game/NPCs/friends/THEKING/HrothgarTalking_InFront.HrothgarTalking_InFront"))
                                          (switch `/Game/dialogueSystem/Enum_Dialogue_State` _state_55
                                            (:`NewEnumerator0`
                                              (bind _state_56 (`self.Add Dialogue` "King Hrothgar" "AAGGGHH! WHY IS HE HERE!?" (`|MakeArray` "Continue" :!type "Text") "/Game/Audio/VoiceLines/KingHrothgar/king-33.king-33" "/Game/NPCs/friends/THEKING/HrothgarTalking_InFront.HrothgarTalking_InFront"))
                                              (switch `/Game/dialogueSystem/Enum_Dialogue_State` _state_56
                                                (:`NewEnumerator0`
                                                  (bind _state_57 (`self.Add Dialogue` "Wiglaf" "W-Well, you sent me to get Beowulf my king! " (`|MakeArray` "Continue" :!type "Text") "/Game/Audio/VoiceLines/wiglaf/wiglaf-07.wiglaf-07" "/Game/NPCs/friends/THEKING/HrothgarTalking_InFront.HrothgarTalking_InFront" (`self.kingAnimationSkeleton`)))
                                                  (switch `/Game/dialogueSystem/Enum_Dialogue_State` _state_57
                                                    (:`NewEnumerator0`
                                                      (bind _state_58 (`self.Add Dialogue` "King Hrothgar" "G-Great! Just fantastic! Great work you two!" (`|MakeArray` "Continue" :!type "Text") "/Game/Audio/VoiceLines/KingHrothgar/king-34.king-34" "/Game/NPCs/friends/THEKING/HrothgarTalking_InFront.HrothgarTalking_InFront"))
                                                      (switch `/Game/dialogueSystem/Enum_Dialogue_State` _state_58
                                                        (:`NewEnumerator0`
                                                          (bind _state_59 (`self.Add Dialogue` "Wiglaf" "T-Thank you, my king! Do you have any more tasks that need doing?" (`|MakeArray` "Continue" :!type "Text") "/Game/Audio/VoiceLines/wiglaf/wiglaf-08.wiglaf-08" "/Game/NPCs/friends/THEKING/HrothgarTalking_InFront.HrothgarTalking_InFront"))
                                                          (switch `/Game/dialogueSystem/Enum_Dialogue_State` _state_59
                                                            (:`NewEnumerator0`
                                                              (bind _state_60 (`self.Add Dialogue` "King Hrothgar" "Uhhhhhhh….." (`|MakeArray` "Continue" :!type "Text") "/Game/Audio/VoiceLines/KingHrothgar/king-35.king-35" "/Game/NPCs/friends/THEKING/HrothgarTalking_InFront.HrothgarTalking_InFront"))
                                                              (switch `/Game/dialogueSystem/Enum_Dialogue_State` _state_60
                                                                (:`NewEnumerator0`
                                                                  (bind _state_61 (`self.Add Dialogue` "King Hrothgar" " For showing how capable you are in both skill and bravery, I want the both of you to…. mow the royal lawn." (`|MakeArray` "Continue" :!type "Text") "/Game/Audio/VoiceLines/KingHrothgar/king-36.king-36" "/Game/NPCs/friends/THEKING/HrothgarTalking_InFront.HrothgarTalking_InFront" (`self.kingAnimationSkeleton`)))
                                                                  (switch `/Game/dialogueSystem/Enum_Dialogue_State` _state_61
                                                                    (:`NewEnumerator0`
                                                                      (bind _state_62 (`self.Add Dialogue` "Beowulf" "Seriously?!" (`|MakeArray` "Continue" :!type "Text") null "/Game/NPCs/friends/THEKING/HrothgarTalking_InFront.HrothgarTalking_InFront"))
                                                                      (switch `/Game/dialogueSystem/Enum_Dialogue_State` _state_62
                                                                        (:`NewEnumerator0`
                                                                          (bind _state_63 (`self.Add Dialogue` "Wiglaf" "YES SIR! I WILL MOW THIS LAWN TO PERFECTION! WOULD YOU ALSO LIKE ME TO LICK YOUR ROYAL BOOTS CLEAN, MY KING?" (`|MakeArray` "Continue" :!type "Text") "/Game/Audio/VoiceLines/wiglaf/wiglaf-09.wiglaf-09" "/Game/NPCs/friends/THEKING/HrothgarTalking_InFront.HrothgarTalking_InFront"))
                                                                          (switch `/Game/dialogueSystem/Enum_Dialogue_State` _state_63
                                                                            (:`NewEnumerator0`
                                                                              (bind _state_64 (`self.Add Dialogue` "King Hrothgar" "Uhm, no Wiglaf, that’s… no." (`|MakeArray` "Continue" :!type "Text") "/Game/Audio/VoiceLines/KingHrothgar/king-37.king-37" "/Game/NPCs/friends/THEKING/HrothgarTalking_InFront.HrothgarTalking_InFront"))
                                                                              (switch `/Game/dialogueSystem/Enum_Dialogue_State` _state_64
                                                                                (:`NewEnumerator0`
                                                                                  (bind _state_65 (`self.Add Dialogue` "Sir Aeschere" "My liege, with all due respect, I think we should use these two for more important tasks than delegating them to plucking grass." (`|MakeArray` "Continue" :!type "Text") null "/Game/NPCs/friends/THEKING/HrothgarTalking_InFront.HrothgarTalking_InFront"))
                                                                                  (switch `/Game/dialogueSystem/Enum_Dialogue_State` _state_65
                                                                                    (:`NewEnumerator0`
                                                                                      (bind _state_66 (`self.Add Dialogue` "Sir Aeschere" "They have both shown themselves to be quite capable, and we haven’t had competent men in well… a milenia. At the very least put them under my command, so that I can make use of them, my lord." (`|MakeArray` "Continue" :!type "Text") null "/Game/NPCs/friends/THEKING/HrothgarTalking_InFront.HrothgarTalking_InFront"))
                                                                                      (switch `/Game/dialogueSystem/Enum_Dialogue_State` _state_66
                                                                                        (:`NewEnumerator0`
                                                                                          (bind _state_67 (`self.Add Dialogue` "King Hrothgar" "*Sigh* I see what you are saying Aeschere, but… look at them!" (`|MakeArray` "Continue" :!type "Text") "/Game/Audio/VoiceLines/KingHrothgar/king-38.king-38" "/Game/NPCs/friends/THEKING/HrothgarTalking_InFront.HrothgarTalking_InFront" (`self.kingAnimationSkeleton`)))
                                                                                          (switch `/Game/dialogueSystem/Enum_Dialogue_State` _state_67
                                                                                            (:`NewEnumerator0`
                                                                                              (bind _state_68 (`self.Add Dialogue` "King Hrothgar" "These dirt ridden- filth peasants have no place in the royal army! I mean… look at that one over there!" (`|MakeArray` "Continue" :!type "Text") "/Game/Audio/VoiceLines/KingHrothgar/king-39.king-39" "/Game/NPCs/friends/THEKING/HrothgarTalking_InFront.HrothgarTalking_InFront"))
                                                                                              (switch `/Game/dialogueSystem/Enum_Dialogue_State` _state_68
                                                                                                (:`NewEnumerator0`
                                                                                                  (bind _state_69 (`self.Add Dialogue` "Wiglaf" " I LOVE GRASS!" (`|MakeArray` "Continue" :!type "Text") "/Game/Audio/VoiceLines/wiglaf/wiglaf-10.wiglaf-10" "/Game/NPCs/friends/THEKING/HrothgarTalking_InFront.HrothgarTalking_InFront"))
                                                                                                  (switch `/Game/dialogueSystem/Enum_Dialogue_State` _state_69
                                                                                                    (:`NewEnumerator0`
                                                                                                      (bind _state_70 (`self.Add Dialogue` "King Hrothgar" "*disgust* Eugh!" (`|MakeArray` "Continue" :!type "Text") "/Game/Audio/VoiceLines/KingHrothgar/king-40.king-40" "/Game/NPCs/friends/THEKING/HrothgarTalking_InFront.HrothgarTalking_InFront"))
                                                                                                      (switch `/Game/dialogueSystem/Enum_Dialogue_State` _state_70
                                                                                                        (:`NewEnumerator0`
                                                                                                          (bind _state_71 (`self.Add Dialogue` "Sir Aeschere" " All I’m asking is to give me a chance to refine them, my liege and if I fail, then I will personally remove them from the royal castle." (`|MakeArray` "Continue" :!type "Text") null "/Game/NPCs/friends/THEKING/HrothgarTalking_InFront.HrothgarTalking_InFront"))
                                                                                                          (switch `/Game/dialogueSystem/Enum_Dialogue_State` _state_71
                                                                                                            (:`NewEnumerator0`
                                                                                                              (bind _state_72 (`self.Add Dialogue` "King Hrothgar" "Hmmm… Ok you got a deal Aeschere. Do with them what you will." (`|MakeArray` "Continue" :!type "Text") "/Game/Audio/VoiceLines/KingHrothgar/king-41.king-41" "/Game/NPCs/friends/THEKING/HrothgarTalking_InFront.HrothgarTalking_InFront"))
                                                                                                              (switch `/Game/dialogueSystem/Enum_Dialogue_State` _state_72
                                                                                                                (:`NewEnumerator0`
                                                                                                                  (bind _state_73 (`self.Add Dialogue` "Sir Aeschere" "You won’t regret this my lord!" (`|MakeArray` "Continue" :!type "Text") null "/Game/NPCs/friends/THEKING/HrothgarTalking_InFront.HrothgarTalking_InFront"))
                                                                                                                  (switch `/Game/dialogueSystem/Enum_Dialogue_State` _state_73
                                                                                                                    (:`NewEnumerator0`
                                                                                                                      (bind _state_74 (`self.Add Dialogue` "Sir Aeschere" "Okay you two, I want you to mee-" (`|MakeArray` "Continue" :!type "Text") null "/Game/NPCs/friends/THEKING/HrothgarTalking_InFront.HrothgarTalking_InFront"))
                                                                                                                      (switch `/Game/dialogueSystem/Enum_Dialogue_State` _state_74
                                                                                                                        (:`NewEnumerator0`
                                                                                                                          (if (not (`self.sceneActionTwo`))
                                                                                                                            (`SceneComponent.K2_SetWorldLocation` (`Actor.RootComponent` _returnvalue_2) (-15983.704597 -31953.397706 200.0) false true)
                                                                                                                            (`/Game/NPCs/foes/GrendelMother/GRENDELMOMMEADHALL.walkInScene` _returnvalue_2)
                                                                                                                            (set `self.sceneActionTwo` true))
                                                                                                                          (bind _state_75 (`self.Add Dialogue` "Grendel's Mother" "Hello false king." (`|MakeArray` "Continue" :!type "Text") "/Game/Audio/VoiceLines/grendelMom/grendelMom-01.grendelMom-01" "/Game/NPCs/friends/THEKING/HrothgarTalking_InFront.HrothgarTalking_InFront"))
                                                                                                                          (switch `/Game/dialogueSystem/Enum_Dialogue_State` _state_75
                                                                                                                            (:`NewEnumerator0`
                                                                                                                              (bind _state_76 (`self.Add Dialogue` "King Hrothgar" "W-WITCH!" (`|MakeArray` "Continue" :!type "Text") "/Game/Audio/VoiceLines/KingHrothgar/king-42.king-42" "/Game/NPCs/friends/THEKING/HrothgarTalking_InFront.HrothgarTalking_InFront"))
                                                                                                                              (switch `/Game/dialogueSystem/Enum_Dialogue_State` _state_76
                                                                                                                                (:`NewEnumerator0`
                                                                                                                                  (bind _state_77 (`self.Add Dialogue` "Grendel's Mother" "Are those your last words? " (`|MakeArray` "Continue" :!type "Text") "/Game/Audio/VoiceLines/grendelMom/grendelMom-02.grendelMom-02" "/Game/NPCs/friends/THEKING/HrothgarTalking_InFront.HrothgarTalking_InFront"))
                                                                                                                                  (switch `/Game/dialogueSystem/Enum_Dialogue_State` _state_77
                                                                                                                                    (:`NewEnumerator0`
                                                                                                                                      (if (not (`self.sceneActionThree`))
                                                                                                                                        (`SkeletalMeshComponent.PlayAnimation` (`self.knightAnimationSkeleton`) "/Game/NPCs/friends/Aeschere/saveTHEKING.saveTHEKING" false)
                                                                                                                                        (`SkeletalMeshComponent.PlayAnimation` (`Character.Mesh` _returnvalue_2) "/Game/NPCs/foes/GrendelMother/Magic_Spell_Casting.Magic_Spell_Casting" false)
                                                                                                                                        (set `self.sceneActionThree` true))
                                                                                                                                      (bind _state_78 (`self.Add Dialogue` "Sir Aeschere" "MY LORD, GET DOWN!" (`|MakeArray` "Continue" :!type "Text") null "/Game/NPCs/friends/Aeschere/saveTHEKING.saveTHEKING" (`self.knightAnimationSkeleton`)))
                                                                                                                                      (switch `/Game/dialogueSystem/Enum_Dialogue_State` _state_78
                                                                                                                                        (:`NewEnumerator0`
                                                                                                                                          (bind _state_79 (`self.Add Dialogue` "King Hrothgar" "AESCHERE!!" (`|MakeArray` "Continue" :!type "Text") "/Game/Audio/VoiceLines/KingHrothgar/king-43.king-43" "/Game/NPCs/friends/THEKING/HrothgarTalking_InFront.HrothgarTalking_InFront"))
                                                                                                                                          (switch `/Game/dialogueSystem/Enum_Dialogue_State` _state_79
                                                                                                                                            (:`NewEnumerator0`
                                                                                                                                              (bind _state_80 (`self.Add Dialogue` "Grendel's Mother" "I’ll be taking this, just as you took something of mine." (`|MakeArray` "Continue" :!type "Text") "/Game/Audio/VoiceLines/grendelMom/grendelMom-03.grendelMom-03" "/Game/NPCs/friends/THEKING/HrothgarTalking_InFront.HrothgarTalking_InFront"))
                                                                                                                                              (`PrimitiveComponent.SetSimulatePhysics` (`Character.Mesh` _asnpc_knight) true)
                                                                                                                                              (switch `/Game/dialogueSystem/Enum_Dialogue_State` _state_80
                                                                                                                                                (:`NewEnumerator0`
                                                                                                                                                  (bind _state_81 (`self.Add Dialogue` "King Hrothgar" "YOU’LL PAY FOR THIS!" (`|MakeArray` "Continue" :!type "Text") "/Game/Audio/VoiceLines/KingHrothgar/king-44.king-44" "/Game/NPCs/friends/THEKING/HrothgarTalking_InFront.HrothgarTalking_InFront"))
                                                                                                                                                  (switch `/Game/dialogueSystem/Enum_Dialogue_State` _state_81
                                                                                                                                                    (:`NewEnumerator0`
                                                                                                                                                      (bind _state_82 (`self.Add Dialogue` "Grendel's Mother" "Goodbye, false king." (`|MakeArray` "Continue" :!type "Text") "/Game/Audio/VoiceLines/grendelMom/grendelMom-04.grendelMom-04" "/Game/NPCs/friends/THEKING/HrothgarTalking_InFront.HrothgarTalking_InFront"))
                                                                                                                                                      (switch `/Game/dialogueSystem/Enum_Dialogue_State` _state_82
                                                                                                                                                        (:`NewEnumerator0`
                                                                                                                                                          (if (not (`self.sceneActionFive`))
                                                                                                                                                            (`/Game/NPCs/foes/GrendelMother/GRENDELMOMMEADHALL.walkOutScene` _returnvalue_2)
                                                                                                                                                            (set `self.sceneActionFive` true))
                                                                                                                                                          (bind _state_83 (`self.Add Dialogue` "King Hrothgar" "ARRRRG!!" (`|MakeArray` "Continue" :!type "Text") "/Game/Audio/VoiceLines/KingHrothgar/king-45.king-45" "/Game/NPCs/friends/THEKING/HrothgarTalking_InFront.HrothgarTalking_InFront"))
                                                                                                                                                          (switch `/Game/dialogueSystem/Enum_Dialogue_State` _state_83
                                                                                                                                                            (:`NewEnumerator0`
                                                                                                                                                              (bind _state_84 (`self.Add Dialogue` "King Hrothgar" "YOU TWO!" (`|MakeArray` "Continue" :!type "Text") "/Game/Audio/VoiceLines/KingHrothgar/king-46.king-46" "/Game/NPCs/friends/THEKING/HrothgarTalking_InFront.HrothgarTalking_InFront"))
                                                                                                                                                              (switch `/Game/dialogueSystem/Enum_Dialogue_State` _state_84
                                                                                                                                                                (:`NewEnumerator0`
                                                                                                                                                                  (bind _state_85 (`self.Add Dialogue` "King Hrothgar" "WIGLAF, KEEP MOWING THAT LAWN!" (`|MakeArray` "Continue" :!type "Text") "/Game/Audio/VoiceLines/KingHrothgar/king-47.king-47" "/Game/NPCs/friends/THEKING/HrothgarTalking_InFront.HrothgarTalking_InFront"))
                                                                                                                                                                  (switch `/Game/dialogueSystem/Enum_Dialogue_State` _state_85
                                                                                                                                                                    (:`NewEnumerator0`
                                                                                                                                                                      (bind _state_86 (`self.Add Dialogue` "King Hrothgar" "BEOWULF!" (`|MakeArray` "Continue" :!type "Text") "/Game/Audio/VoiceLines/KingHrothgar/king-48.king-48" "/Game/NPCs/friends/THEKING/HrothgarTalking_InFront.HrothgarTalking_InFront"))
                                                                                                                                                                      (switch `/Game/dialogueSystem/Enum_Dialogue_State` _state_86
                                                                                                                                                                        (:`NewEnumerator0`
                                                                                                                                                                          (bind _state_87 (`self.Add Dialogue` "King Hrothgar" "THAT WOMAN LIVES IN THE LAKE PAST THE MOUNTAINS!" (`|MakeArray` "Continue" :!type "Text") "/Game/Audio/VoiceLines/KingHrothgar/king-49.king-49" "/Game/NPCs/friends/THEKING/HrothgarTalking_InFront.HrothgarTalking_InFront" :!label _label_2))
                                                                                                                                                                          (switch `/Game/dialogueSystem/Enum_Dialogue_State` _state_87
                                                                                                                                                                            (:`NewEnumerator0`
                                                                                                                                                                              (bind _state_88 (`self.Add Dialogue` "King Hrothgar" "GO GET THAT WITCH AND EXECUTE HER THIS INSTANT!" (`|MakeArray` "Continue" :!type "Text") "/Game/Audio/VoiceLines/KingHrothgar/king-50.king-50" "/Game/NPCs/friends/THEKING/HrothgarTalking_InFront.HrothgarTalking_InFront"))
                                                                                                                                                                              (switch `/Game/dialogueSystem/Enum_Dialogue_State` _state_88
                                                                                                                                                                                (:`NewEnumerator0`
                                                                                                                                                                                  (bind _state_89 (`self.Add Dialogue` "King Hrothgar" "THAT’S AN ORDER!" (`|MakeArray` "Continue" :!type "Text") "/Game/Audio/VoiceLines/KingHrothgar/king-51.king-51" "/Game/NPCs/friends/THEKING/HrothgarTalking_InFront.HrothgarTalking_InFront"))
                                                                                                                                                                                  (switch `/Game/dialogueSystem/Enum_Dialogue_State` _state_89
                                                                                                                                                                                    (:`NewEnumerator0`
                                                                                                                                                                                      (`self.setDialogueTreeIndex` 3)
                                                                                                                                                                                      (set `self.dialogueTreeIndex` 3)
                                                                                                                                                                                      (`self.closeConvo`)
                                                                                                                                                                                      (`self.clearDialogueProgress`)
                                                                                                                                                                                      (bind _firstpersoncamera (`/Game/Dynamic/FirstPerson/Blueprints/BP_FirstPersonCharacter.FirstPersonCamera` _asbp_first_person_character))
                                                                                                                                                                                      (`CameraComponent.GetCameraView` _firstpersoncamera 0.0)
                                                                                                                                                                                      (`PlayerController.SetViewTargetWithBlend` (`GameplayStatics.GetPlayerController` 0) (`self.GetOwner` _firstpersoncamera) 0.0 "VTBlend_Linear" 0.0 false)
                                                                                                                                                                                      (bind _as_level_save_data_2 (`/Game/Dynamic/FirstPerson/Blueprints/BP_FirstPersonGameMode.As Level Save Data` _game_mode))
                                                                                                                                                                                      (set `/Game/Dynamic/FirstPerson/Blueprints/levelSaveData.kingDialogueTreeIndex` 3 _as_level_save_data_2)
                                                                                                                                                                                      (set `/Game/Dynamic/FirstPerson/Blueprints/levelSaveData.questGiveGrendelMother?` true _as_level_save_data_2))))))))))))))))))))))))))))))))))))))))))))))))))))))))))))))))))))))))))))))))))))))))))
    (:`3`
      (goto _label_2))))