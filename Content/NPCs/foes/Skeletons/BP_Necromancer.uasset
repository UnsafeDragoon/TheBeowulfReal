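; Necromancer enemy that roams randomly, chases the player and makes timed area attacks that damage and launch them upward.
; Tick updates a camera-facing health bar and checks narrow distance bands to start or stop pursuit, otherwise roaming when idle.
; ChaseBeowulf loops AI MoveTo, then briefly enables AttackCollision with an explosion sound.
; Incoming damage reduces health, ending in ragdoll and delayed destruction.
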(event `roamAround`
  (bind (_returnvalue_x _returnvalue_y _returnvalue_z) (`KismetMathLibrary.BreakVector` (`SceneComponent.K2_GetComponentLocation` (`self.SkeletalMesh`))))
  ;[1 0 0.6548] Roam Around Open World (Not in pursuit)
  (set `CharacterMovementComponent.MaxWalkSpeed` 50.0 (`self.CharacterMovement`))
  (set `self.randomMove?` false)
  (`|AIMoveTo` self (`KismetMathLibrary.MakeVector` (+ _returnvalue_x (* (`KismetMathLibrary.RandomFloatInRange` 200.0 600.0) (`KismetMathLibrary.SignOfFloat` (`KismetMathLibrary.RandomFloatInRange` -5.0 5.0)))) (+ _returnvalue_y (* (`KismetMathLibrary.RandomFloatInRange` 200.0 600.0) (`KismetMathLibrary.SignOfFloat` (`KismetMathLibrary.RandomFloatInRange` -5.0 5.0)))) (+ _returnvalue_z 100.0)) null
    (:`then`
      (`KismetSystemLibrary.Delay` 5.0)
      (set `self.randomMove?` true))))

(event `ChaseBeowulf`
  ;[1 0 0.6634] CHASE THE PLAYER
  (set `self.chasingPlayer?` true)
  (set `CharacterMovementComponent.MaxWalkSpeed` 300.0 (`self.CharacterMovement`))
  (bind _asbp_first_person_character (cast `/Game/Dynamic/FirstPerson/Blueprints/BP_FirstPersonCharacter` (`GameplayStatics.GetPlayerCharacter` 0)))
  (if (not (`/Game/Dynamic/FirstPerson/Blueprints/BP_FirstPersonCharacter.isDead` _asbp_first_person_character))
    (`|AIMoveTo` self (0.0 0.0 0.0) (`GameplayStatics.GetPlayerCharacter` 0) 1500.0
      (:`OnSuccess`
        (bind _output_get (set `self.Target` (`KismetMathLibrary.RandomIntegerInRange` 0 1)))
        (set `self.IsAttacking?` true)
        (if (== _output_get 0)
          _
          (else
            _))
        (`KismetSystemLibrary.Delay` 1.15)
        (`GameplayStatics.PlaySoundAtLocation` "/Game/StarterContent/Audio/Explosion01.Explosion01" (`SceneComponent.K2_GetComponentLocation` (`self.SkeletalMesh`)) (struct) 0.6 1.0 -1.0 null null null null)
        (`PrimitiveComponent.SetCollisionEnabled` (`self.AttackCollision`) "QueryOnly")
        (`KismetSystemLibrary.Delay` 0.6)
        (`PrimitiveComponent.SetCollisionEnabled` (`self.AttackCollision`) "NoCollision")
        (`KismetSystemLibrary.Delay` 1.8)
        (set `self.IsAttacking?` false)
        (`self.ChaseBeowulf`)))))

(event `self.ReceiveTick`
  (params (DeltaSeconds :type "Float (single-precision)"))
  (bind _charactermovement (`self.CharacterMovement`))
  (bind _healthbarwidget (`self.healthBarWidget`))
  (bind (_returnvalue_x _returnvalue_y) (`KismetMathLibrary.BreakVector` (`SceneComponent.K2_GetComponentLocation` (`self.SkeletalMesh`))))
  ;[1 0 0.5968] Check If Player is in detection range
  ;[1 0 0.6185] Real Time World Health Bar
  (bind _aswb_enemy_health (cast `/Game/NPCs/foes/WB_EnemyHealth` (`WidgetComponent.GetWidget` (`self.healthBarWidget`))))
  (`ProgressBar.SetPercent` (`/Game/NPCs/foes/WB_EnemyHealth.healthBar` _aswb_enemy_health) (/ (`self.Health`) 200.0))
  (`SceneComponent.K2_SetWorldRotation` _healthbarwidget (`KismetMathLibrary.FindLookAtRotation` (`SceneComponent.K2_GetComponentLocation` _healthbarwidget) (`SceneComponent.K2_GetComponentLocation` (`PlayerCameraManager.TransformComponent` (`GameplayStatics.GetPlayerCameraManager` 0)))) false false)
  (bind _asbp_first_person_character (cast `/Game/Dynamic/FirstPerson/Blueprints/BP_FirstPersonCharacter` (`GameplayStatics.GetPlayerCharacter` 0)))
  (bind (_returnvalue_x_2 _returnvalue_y_2) (`KismetMathLibrary.BreakVector` (`SceneComponent.K2_GetComponentLocation` (`Character.CapsuleComponent` _asbp_first_person_character))))
  (bind _returnvalue (`KismetMathLibrary.Sqrt` (+ (`KismetMathLibrary.Square` (`KismetMathLibrary.Abs` (- _returnvalue_y_2 _returnvalue_y))) (`KismetMathLibrary.Square` (`KismetMathLibrary.Abs` (- _returnvalue_x_2 _returnvalue_x))))))
  (if (and (<= _returnvalue 3522.0) (>= _returnvalue 3422.0))
    (set `self.chasingPlayer?` false)
    (`NavMovementComponent.StopActiveMovement` _charactermovement)
    (elif (and (>= _returnvalue 1326.0) (<= _returnvalue 1426.0))
      (`self.ChaseBeowulf`)
      (elif (== (`MovementComponent.Velocity` _charactermovement) (0.0 0.0 0.0))
        (if (`self.chasingPlayer?`)
          _
          (elif (and (not (`self.IsAttacking?`)) (`self.randomMove?`))
            (`self.roamAround`)))))))

(event `self.ReceiveBeginPlay`
  ;[1 0 0.6822] Disable Attack Hitbox on spawn
  (`PrimitiveComponent.SetCollisionEnabled` (`self.AttackCollision`) "NoCollision"))

(event `self.AttackCollision.OnComponentBeginOverlap`
  (params (OverlappedComponent :type "PrimitiveComponent Object Reference") (OtherActor :type "Actor Object Reference") (OtherComp :type "PrimitiveComponent Object Reference") (OtherBodyIndex :type Integer) (bFromSweep :type Boolean) (SweepResult :type "HitResult Structure (by ref)"))
  (if (not (== OtherActor self))
    (bind _asbp_first_person_character (cast `/Game/Dynamic/FirstPerson/Blueprints/BP_FirstPersonCharacter` OtherActor))
    ;[1 0 0.5828] AttackHitPlayer
    (if (not (== (`/Game/Dynamic/FirstPerson/Blueprints/BP_FirstPersonCharacter.interactCollision` _asbp_first_person_character) OtherComp))
      (bind _asbp_first_person_character_2 (cast `/Game/Dynamic/FirstPerson/Blueprints/BP_FirstPersonCharacter` (`GameplayStatics.GetPlayerCharacter` 0)))
      (if (not (`/Game/Dynamic/FirstPerson/Blueprints/BP_FirstPersonCharacter.isDead` _asbp_first_person_character_2))
        (`PrimitiveComponent.SetCollisionEnabled` (`self.AttackCollision`) "NoCollision")
        (`GameplayStatics.ApplyDamage` _asbp_first_person_character 100.0)
        (`self.LaunchCharacter` _asbp_first_person_character_2 (0.0 0.0 1000.0) false false)
        (`KismetSystemLibrary.Delay` 3.0)
        (`self.ChaseBeowulf`)))))

(event `self.ReceiveAnyDamage`
  (params (Damage :type "Float (single-precision)") (DamageType :type "DamageType Object Reference") (InstigatedBy :type "Controller Object Reference") (DamageCauser :type "Actor Object Reference"))
  ;[1 0 0.5763] Death
  (bind _output_get (set `self.Health` (- (`self.Health`) Damage)))
  (if (<= _output_get 0.0)
    (`PrimitiveComponent.SetSimulatePhysics` (`self.SkeletalMesh`) true)
    (`CharacterMovementComponent.DisableMovement` (`self.CharacterMovement`))
    (`PrimitiveComponent.SetCollisionEnabled` (`self.AttackCollision`) "NoCollision")
    (`KismetSystemLibrary.Delay` 5.0)
    (`self.K2_DestroyActor`)))

(event `self.characterCollision.OnComponentBeginOverlap`
  (params (OverlappedComponent :type "PrimitiveComponent Object Reference") (OtherActor :type "Actor Object Reference") (OtherComp :type "PrimitiveComponent Object Reference") (OtherBodyIndex :type Integer) (bFromSweep :type Boolean) (SweepResult :type "HitResult Structure (by ref)")))

(fn `staminaDrain`)

(fn `UserConstructionScript`)